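; BP_SHUD is a HUD Blueprint that draws a dynamic crosshair and creates the main HUD layout widget.
; On BeginPlay it creates WBP_HUDLayout, stores the reference and adds it to the viewport.
; Each frame, DrawHUD draws four rotated copies of one line texture around screen centre, spread by scaled PlayerSpeed plus TargetingModifier.
; Neither spread variable is set within this graph.
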(event EventBeginPlay
  (Utilities|FlowControl|Sequence
    (:then_0
      (bind _returnvalue (UserInterface|CreateWidget "/Game/UI/WBP_HUDLayout.WBP_HUDLayout_C"))
      (bind _output_get (Variables|Default|SetHUDLayoutWidget _returnvalue))
      (UserInterface|Viewport|AddtoViewport _output_get 0))))

(event EventDrawHUD
  (params (SizeX :type Integer) (SizeY :type Integer))
  (bind _targeting_modifier (Variables|Default|GetTargeting%20Modifier))
  (bind _playerspeed (Variables|Default|GetPlayerSpeed))
  (bind _returnvalue (/ _playerspeed 35.0))
  (bind _returnvalue_2 (+ _returnvalue _targeting_modifier))
  ;[1 1 1] Draw Crosshair
  (Variables|Default|SetScreenX (Math|Conversions|ToFloat(Integer) (/ SizeX 2)))
  (Variables|Default|SetScreenY (Math|Conversions|ToFloat(Integer) (/ SizeY 2)))
  (Canvas|DrawTexture "/Game/Base/Crosshair/T_TypeA_vert.T_TypeA_vert" (Variables|Default|GetScreenX) (+ (Variables|Default|GetScreenY) _returnvalue_2) 1.0 1e+01 0.0 0.0 1.0 1.0 "(R=1.000000,G=1.000000,B=1.000000,A=1.000000)") ; Bottom
  (Canvas|DrawTexture "/Game/Base/Crosshair/T_TypeA_vert.T_TypeA_vert" (- (Variables|Default|GetScreenX) _returnvalue_2) (Variables|Default|GetScreenY) 1.0 1e+01 0.0 0.0 1.0 1.0 "(R=1.000000,G=1.000000,B=1.000000,A=1.000000)" "BLEND_Translucent" 1.0 false 9e+01) ; Left
  (Canvas|DrawTexture "/Game/Base/Crosshair/T_TypeA_vert.T_TypeA_vert" (+ (Variables|Default|GetScreenX) _returnvalue_2) (Variables|Default|GetScreenY) -1.0 1e+01 0.0 0.0 1.0 1.0 "(R=1.000000,G=1.000000,B=1.000000,A=1.000000)" "BLEND_Translucent" 1.0 false -9e+01 "(X=0.000000,Y=0.000000)") ; Right
  (Canvas|DrawTexture "/Game/Base/Crosshair/T_TypeA_vert.T_TypeA_vert" (Variables|Default|GetScreenX) (- (Variables|Default|GetScreenY) _returnvalue_2) -1.0 1e+01 0.0 0.0 1.0 1.0 "(R=1.000000,G=1.000000,B=1.000000,A=1.000000)" "BLEND_Translucent" 1.0 false 1.8e+02) ; Top
)

(fn ConstructionScript)